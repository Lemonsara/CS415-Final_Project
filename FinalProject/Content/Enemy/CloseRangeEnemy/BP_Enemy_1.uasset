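; BP_Enemy_1 is a close-range enemy that chases the player once seen and otherwise advances on the scene's FbxScene_ZenUV_SciFi_TrimSheet_01 actor.
; PawnSensing feeds the FollowPlayer AIMoveTo loop; on arrival it plays an attack montage, waiting out its length as cooldown.
; Each attack damages that scene actor, even when the player is the move target.
; AnyDamage lowers BloodNow, exposed through GetHP alongside an owner-linked BloodBar widget, and destroys the enemy at zero.
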(event `self.ReceiveTick`
  (params (DeltaSeconds :type "Float (single-precision)")))

(event `self.ReceiveBeginPlay`
  (bind _aswb_blood_bar (cast `/Game/Enemy/CloseRangeEnemy/WB_BloodBar` (`WidgetComponent.GetUserWidgetObject` (`self.BloodBar`))))
  (set `/Game/Enemy/CloseRangeEnemy/WB_BloodBar.Enemyowner` self _aswb_blood_bar)
  (bind _returnvalue (`GameplayStatics.GetActorOfClass` "/Game/Others_imported/FbxScene_ZenUV_SciFi_TrimSheet_01.FbxScene_ZenUV_SciFi_TrimSheet_01_C"))
  (set `self.FBX` _returnvalue)
  (`self.FollowPlayer`))

(event `self.PawnSensing.OnSeePawn`
  (params (Pawn :type "Pawn Object Reference"))
  (set `self.isSeeingPlayer` (== Pawn (`GameplayStatics.GetPlayerPawn` 0)))
  (`self.FollowPlayer`))

(event `FollowPlayer`
  (bind (_returnvalue_roll _returnvalue_pitch _returnvalue_yaw) (`KismetMathLibrary.BreakRotator` (`KismetMathLibrary.FindLookAtRotation` (`self.K2_GetActorLocation`) (`self.K2_GetActorLocation` (`self.FBX`)))))
  (if (`self.isSeeingPlayer`)
    (`|AIMoveTo` self (0.0 0.0 0.0) (`GameplayStatics.GetPlayerPawn` 0) 70.0
      (:`OnSuccess`
        (if (`self.canAttack`) :!label _label
          (set `self.canAttack` false)
          (bind _returnvalue (`self.PlayAnimMontage` "/Game/Enemy/Animation/AI/AttackAnimMontage.AttackAnimMontage"))
          (`KismetSystemLibrary.RetriggerableDelay` _returnvalue)
          (set `self.canAttack` true)
          (bind _returnvalue_2 (`GameplayStatics.GetActorOfClass` "/Game/Others_imported/FbxScene_ZenUV_SciFi_TrimSheet_01.FbxScene_ZenUV_SciFi_TrimSheet_01_C"))
          (`GameplayStatics.ApplyDamage` _returnvalue_2 20.0)
          (`KismetSystemLibrary.PrintString` "wtf")
          (`self.FollowPlayer`))))
    (else
      (set `self.isSeeingPlayer` false)
      (`self.FBX`
        (:`then`
          (`|AIMoveTo` self (0.0 0.0 0.0) (`self.FBX`) 800.0
            (:`then`
              (`self.K2_SetActorRotation` self (`KismetMathLibrary.MakeRotator` 0.0 0.0 _returnvalue_yaw) false))
            (:`OnSuccess`
              (goto _label))))
        (:`else`
          (`self.FollowPlayer`))))))

(event `/Game/Enemy/CloseRangeEnemy/BPI_Enemy.EnemyHit`
  (params (Damage :type "Float (double-precision)"))
  (bind _output_get (set `self.BloodNow` (`KismetMathLibrary.FClamp` (- (`self.BloodNow`) Damage) 0.0 (`self.BloodMax`))))
  (if (<= _output_get 0.0)
    (`self.K2_DestroyActor`)))

(event `self.ReceiveAnyDamage`
  (params (Damage :type "Float (single-precision)") (DamageType :type "DamageType Object Reference") (InstigatedBy :type "Controller Object Reference") (DamageCauser :type "Actor Object Reference"))
  (`self.EnemyHit` Damage))

(fn `GetHP`
  (returns (NOW :type "Float (double-precision)") (MAX :type "Float (double-precision)"))
  (return (`self.BloodNow`) (`self.BloodMax`)))

(fn `UserConstructionScript`)