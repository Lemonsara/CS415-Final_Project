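; BP_RemoteEnemy is a ranged grenadier enemy that approaches the player and throws BP_Boom.
; Pawn sensing sets IsSeeingPlayer, which is never cleared, and starts an AI move to within range.
; On arrival, CanAttack gates a throw montage and a delayed spawn at the right-hand socket.
; EnemyHit reduces health and destroys the actor at zero; a WB_BloodBar widget gets it as owner.
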(event `self.ReceiveTick`
  (params (DeltaSeconds :type "Float (single-precision)"))
  (if (not (`self.isSeeingPlayer`))
    (`MovementComponent.StopMovementImmediately` (`self.CharacterMovement`))))

(event `self.ReceiveBeginPlay`
  (bind _aswb_blood_bar (cast `/Game/Enemy/CloseRangeEnemy/WB_BloodBar` (`WidgetComponent.GetUserWidgetObject` (`self.BloodBar`))))
  (set `/Game/Enemy/CloseRangeEnemy/WB_BloodBar.Enemyowner` self _aswb_blood_bar))

(event `self.PawnSensing.OnSeePawn`
  (params (Pawn :type "Pawn Object Reference"))
  (`KismetSystemLibrary.PrintString` "see u")
  (set `self.isSeeingPlayer` true)
  (`self.FollowPlayer`))

(event `FollowPlayer`
  (bind _returnvalue (`GameplayStatics.GetPlayerPawn` 0))
  (if (`self.isSeeingPlayer`)
    (if (`self.canAttack`)
      (`|AIMoveTo` self (0.0 0.0 0.0) _returnvalue 500.0
        (:`then`
          (`self.K2_SetActorRotation` (`KismetMathLibrary.FindLookAtRotation` (`self.K2_GetActorLocation` self) (`self.K2_GetActorLocation` _returnvalue))))
        (:`OnSuccess`
          (if (`self.canAttack`)
            (set `self.canAttack` false)
            (bind _returnvalue_2 (`self.PlayAnimMontage` "/Game/CityofBrass_Enemies/Meshes/Enemy/Grenadier/Animation/Grenadier_Attack_Throw_Montage.Grenadier_Attack_Throw_Montage"))
            (`|ExecutionSequence`
              (:`then_0`
                (`KismetSystemLibrary.RetriggerableDelay` _returnvalue_2)
                (set `self.canAttack` true))
              (:`then_1`
                (`KismetSystemLibrary.RetriggerableDelay` 0.7)
                (`|SpawnActorFromClass` "/Game/Enemy/RemoteEnemy/BP_Boom.BP_Boom_C" (`KismetMathLibrary.MakeTransform` (`SceneComponent.GetSocketLocation` (`self.Mesh`) "Bip001-R-Hand") (`self.K2_GetActorRotation`)) "AlwaysSpawn" "MultiplyWithRoot" null null null)))))))))

(event `/Game/Enemy/CloseRangeEnemy/BPI_Enemy.EnemyHit`
  (params (Damage :type "Float (double-precision)"))
  (bind _output_get (set `self.BloodNow` (`KismetMathLibrary.FClamp` (- (`self.BloodNow`) Damage) 0.0 (`self.BloodMax`))))
  (if (<= _output_get 0.0)
    (`self.K2_DestroyActor`)))

(event `self.ReceiveAnyDamage`
  (params (Damage :type "Float (single-precision)") (DamageType :type "DamageType Object Reference") (InstigatedBy :type "Controller Object Reference") (DamageCauser :type "Actor Object Reference")))

(fn `GetHP`
  (returns (NOW :type "Float (double-precision)") (MAX :type "Float (double-precision)"))
  (return (`self.BloodNow`) (`self.BloodMax`)))

(fn `UserConstructionScript`)