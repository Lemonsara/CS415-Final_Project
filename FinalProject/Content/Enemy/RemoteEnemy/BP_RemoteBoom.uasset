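; Explosive actor for the remote enemy that detonates on contact with anything not implementing BPI_Enemy, or silently destroys itself after three seconds.
; Tick polls FTest, a sphere trace sized by its Sphere component, instead of using overlap events.
; On the first hit, FRang traces for pawns and damages the player or FbxScene_ZenUV_SciFi_TrimSheet_01 actors, then BP_Fire spawns and the actor is destroyed.
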(event `self.ReceiveBeginPlay`
  (`KismetSystemLibrary.Delay` 3.0)
  (`self.K2_DestroyActor`))

(event `self.ReceiveTick`
  (params (DeltaSeconds :type "Float (single-precision)"))
  (bind _hit_ (`self.F_Test`))
  (if _hit_
    (`/Engine/EditorBlueprintResources/StandardMacros.DoOnce` false
      (:`Completed`
        (`self.F_rang`)
        (`|SpawnActorFromClass` "/Game/Enemy/RemoteEnemy/BP_Fire.BP_Fire_C" (`KismetMathLibrary.Conv_VectorToTransform` (`self.K2_GetActorLocation`)) "AlwaysSpawn" "MultiplyWithRoot" null null)
        (`self.K2_DestroyActor`)))))

(fn `F_rang`
  (bind _returnvalue (`self.K2_GetActorLocation`))
  (bind _returnvalue_2 (`GameplayStatics.GetPlayerPawn` 0))
  (bind _outhits (`KismetSystemLibrary.SphereTraceMultiForObjects` _returnvalue _returnvalue (`SphereComponent.SphereRadius` (`self.Sphere`)) (`|MakeArray` "ObjectTypeQuery3" :!type "EObjectTypeQuery Enum")))
  (for _array_element _outhits
    (bind (_bblockinghit _binitialoverlap _time _distance _location _impactpoint _normal _impactnormal _physmat _hitactor) (`GameplayStatics.BreakHitResult` _array_element))
    (if (== _hitactor _returnvalue_2)
      (bind _asbp_first_person_character (cast `/Game/FirstPerson/Blueprints/BP_FirstPersonCharacter` _returnvalue_2))
      (`GameplayStatics.ApplyDamage` _asbp_first_person_character (`self.Damage`) null self)
      (break)
      (else
        (bind _asfbx_scene_zen_uv_sci_fi_trim_sheet_01 (cast `/Game/Others_imported/FbxScene_ZenUV_SciFi_TrimSheet_01` _hitactor))
        (`GameplayStatics.ApplyDamage` _asfbx_scene_zen_uv_sci_fi_trim_sheet_01 (`self.Damage`)))))
  (return))

(fn `F_Test`
  (returns (`Hit？` :type Boolean))
  (locals (`hit?` :type Boolean :default false))
  (bind _returnvalue (`self.K2_GetActorLocation`))
  (bind (_outhits _returnvalue_2) (`KismetSystemLibrary.SphereTraceMultiForObjects` _returnvalue _returnvalue (`SphereComponent.SphereRadius` (`self.Sphere`)) (`|MakeArray` "ObjectTypeQuery3" "ObjectTypeQuery1" "ObjectTypeQuery2" :!type "EObjectTypeQuery Enum")))
  (if _returnvalue_2
    (for _array_element _outhits
      (if (not (`KismetSystemLibrary.DoesImplementInterface` (`.HitActor` (`GameplayStatics.BreakHitResult` _array_element)) "/Game/Enemy/CloseRangeEnemy/BPI_Enemy.BPI_Enemy_C"))
        (set `local.hit?` true)))
    (return (`local.hit?`))
    (else
      (return (`local.hit?`)))))

(fn `UserConstructionScript`)