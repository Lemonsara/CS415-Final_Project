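; BP_Enemy_1_Child is an exploding enemy variant that closes on a target and self-destructs.
; Its FollowPlayer event uses AI MoveTo toward the player when seen, otherwise toward the FBX target if valid.
; On arrival it spawns BP_Boom, calls FRang and destroys itself.
; FRang runs a debug-drawn sphere trace for pawns, applying BaseDamage to the player or FbxScene_ZenUV_SciFi_TrimSheet_01 hits, stopping once it hits the player.
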(event `self.FollowPlayer`
  (if (`self.isSeeingPlayer`)
    (`|AIMoveTo` self (0.0 0.0 0.0) (`GameplayStatics.GetPlayerPawn` 0) 350.0 true
      (:`OnSuccess`
        _))
    (else
      (`self.FBX`
        (:`then`
          (`|AIMoveTo` self (0.0 0.0 0.0) (`self.FBX`) 600.0
            (:`OnSuccess`
              _)))
        (:`else`))))
  (`|SpawnActorFromClass` "/Game/Enemy/BoomEnemy/BP_Boom.BP_Boom_C" (`self.GetTransform`) "AlwaysSpawn" "MultiplyWithRoot" null null)
  (`self.F_rang`)
  (`self.K2_DestroyActor`))

(fn `F_rang`
  (bind _returnvalue (`self.K2_GetActorLocation`))
  (bind _returnvalue_2 (`GameplayStatics.GetPlayerPawn` 0))
  (bind _outhits (`KismetSystemLibrary.SphereTraceMultiForObjects` :`Start` _returnvalue :`End` _returnvalue :`Radius` 350.0 :`ObjectTypes` (`|MakeArray` "ObjectTypeQuery3" :!type "EObjectTypeQuery Enum") :`DrawDebugType` "ForDuration"))
  (for _array_element _outhits
    (bind (_bblockinghit _binitialoverlap _time _distance _location _impactpoint _normal _impactnormal _physmat _hitactor) (`GameplayStatics.BreakHitResult` _array_element))
    (if (== _hitactor _returnvalue_2)
      (bind _asbp_first_person_character (cast `/Game/FirstPerson/Blueprints/BP_FirstPersonCharacter` _returnvalue_2))
      (`GameplayStatics.ApplyDamage` _asbp_first_person_character (`self.Base Damage`) null self)
      (break)
      (else
        (bind _asfbx_scene_zen_uv_sci_fi_trim_sheet_01 (cast `/Game/Others_imported/FbxScene_ZenUV_SciFi_TrimSheet_01` _hitactor))
        (`GameplayStatics.ApplyDamage` _asfbx_scene_zen_uv_sci_fi_trim_sheet_01 (`self.Base Damage`)))))
  (return))

(fn `UserConstructionScript`
  (`parent.UserConstructionScript`))