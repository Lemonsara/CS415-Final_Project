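; BP_Magic_Turret is a turret that slows enemies inside its Range component.
; Overlap begin and end events scale MaxWalkSpeed on BP_Enemy_1 or BP_RemoteEnemy, cutting it on entry and raising it on exit.
; The exit multiplier fully restores BP_Enemy_1, but BP_RemoteEnemy is slowed more heavily and leaves below its original speed.
; The graph contains no attack logic.
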(event `self.range.OnComponentBeginOverlap`
  (params (OverlappedComponent :type "PrimitiveComponent Object Reference") (OtherActor :type "Actor Object Reference") (OtherComp :type "PrimitiveComponent Object Reference") (OtherBodyIndex :type Integer) (bFromSweep :type Boolean) (SweepResult :type "HitResult Structure (by ref)"))
  (bind _asbp_enemy_1 (cast `/Game/Enemy/CloseRangeEnemy/BP_Enemy_1` OtherActor)
    (:`then`
      (if (`KismetSystemLibrary.IsValid` _asbp_enemy_1)
        (bind _charactermovement (`Character.CharacterMovement` _asbp_enemy_1))
        (set `CharacterMovementComponent.MaxWalkSpeed` (* (`CharacterMovementComponent.MaxWalkSpeed` _charactermovement) 0.8) _charactermovement)))
    (:`CastFailed`
      (bind _asbp_remote_enemy (cast `/Game/Enemy/RemoteEnemy/BP_RemoteEnemy` OtherActor))
      (if (`KismetSystemLibrary.IsValid` _asbp_remote_enemy)
        (bind _charactermovement_2 (`Character.CharacterMovement` _asbp_remote_enemy))
        (set `CharacterMovementComponent.MaxWalkSpeed` (* (`CharacterMovementComponent.MaxWalkSpeed` _charactermovement_2) 0.5) _charactermovement_2)))))

(event `self.range.OnComponentEndOverlap`
  (params (OverlappedComponent :type "PrimitiveComponent Object Reference") (OtherActor :type "Actor Object Reference") (OtherComp :type "PrimitiveComponent Object Reference") (OtherBodyIndex :type Integer))
  (bind _asbp_enemy_1 (cast `/Game/Enemy/CloseRangeEnemy/BP_Enemy_1` OtherActor)
    (:`then`
      (if (`KismetSystemLibrary.IsValid` _asbp_enemy_1)
        (bind _charactermovement (`Character.CharacterMovement` _asbp_enemy_1))
        (set `CharacterMovementComponent.MaxWalkSpeed` (* (`CharacterMovementComponent.MaxWalkSpeed` _charactermovement) 1.25) _charactermovement)))
    (:`CastFailed`
      (bind _asbp_remote_enemy (cast `/Game/Enemy/RemoteEnemy/BP_RemoteEnemy` OtherActor))
      (if (`KismetSystemLibrary.IsValid` _asbp_remote_enemy)
        (bind _charactermovement_2 (`Character.CharacterMovement` _asbp_remote_enemy))
        (set `CharacterMovementComponent.MaxWalkSpeed` (* (`CharacterMovementComponent.MaxWalkSpeed` _charactermovement_2) 1.25) _charactermovement_2)))))

(fn `UserConstructionScript`)