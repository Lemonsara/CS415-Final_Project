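; Rocket turret actor that automatically finds nearby enemies and hits them with area damage.
; A delayed, self-calling Check scans all BP_Enemy_1, then BP_RemoteEnemy actors, taking the first within that type's range rather than the nearest.
; AttackRound starts a recursive yaw-tracking loop, spawns BP_Rocket_Fire directly on the target and applies instant radial damage, with no projectile travel.
; It repeats on a delay while the target stays valid and in range, otherwise returning to Check.
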(event `self.ReceiveBeginPlay`
  (`self.check`))

(event `check`
  (`KismetSystemLibrary.Delay` 1.5)
  (bind _outactors (`GameplayStatics.GetAllActorsOfClass` "/Game/Enemy/CloseRangeEnemy/BP_Enemy_1.BP_Enemy_1_C"))
  (for _array_element _outactors
    (if (<= (`KismetMathLibrary.VSize` (- (`self.K2_GetActorLocation` _array_element) (`self.K2_GetActorLocation`))) 1500.0)
      (set `self.current_target` _array_element)
      (`self.AttackRound`)
      (break)))
  (bind _outactors_2 (`GameplayStatics.GetAllActorsOfClass` "/Game/Enemy/RemoteEnemy/BP_RemoteEnemy.BP_RemoteEnemy_C"))
  (for _array_element_2 _outactors_2
    (if (<= (`KismetMathLibrary.VSize` (- (`self.K2_GetActorLocation` _array_element_2) (`self.K2_GetActorLocation`))) 2000.0)
      (set `self.current_target` _array_element_2)
      (`self.AttackRound`)
      (break)
      (else
        (`KismetSystemLibrary.Delay` 1.5)
        (`self.check`)
        (break))))
  (`self.check`))

(event `FaceTarget`
  (bind (_returnvalue_roll _returnvalue_pitch _returnvalue_yaw) (`KismetMathLibrary.BreakRotator` (`KismetMathLibrary.RInterpTo` (`self.K2_GetActorRotation`) (`KismetMathLibrary.FindLookAtRotation` (`self.K2_GetActorLocation`) (`self.K2_GetActorLocation` (`self.current_target`))) (`GameplayStatics.GetWorldDeltaSeconds`) 20.0)))
  ;[1 1 1] rotation
  (if (`KismetSystemLibrary.IsValid` (`self.current_target`))
    (`self.K2_SetActorRotation` (`KismetMathLibrary.MakeRotator` 0.0 0.0 _returnvalue_yaw))
    (`KismetSystemLibrary.Delay` 0.05)
    (`self.FaceTarget`)))

(event `AttackRound`
  (if (`KismetSystemLibrary.IsValid` (`self.current_target`))
    (`self.FaceTarget`)
    (`|SpawnActorFromClass` "/Game/Turret/rocket_turret/BP_Rocket_Fire.BP_Rocket_Fire_C" (`KismetMathLibrary.Conv_VectorToTransform` (`self.K2_GetActorLocation` (`self.current_target`))) "Undefined" "MultiplyWithRoot" null null)
    (`GameplayStatics.ApplyRadialDamage` :`BaseDamage` 5.0 :`Origin` (`self.K2_GetActorLocation` (`self.current_target`)) :`DamageRadius` 350.0 :`DamageCauser` null :`InstigatedByController` null)
    (if (`KismetSystemLibrary.IsValid` (`self.current_target`))
      (if (<= (`KismetMathLibrary.VSize` (- (`self.K2_GetActorLocation` (`self.current_target`)) (`self.K2_GetActorLocation`))) 2000.0)
        (`KismetSystemLibrary.Delay` 3.0)
        (`self.AttackRound`)
        (else
          (`self.check`)))
      (else
        (`self.check`)))
    (else
      (`self.check`))))

(fn `UserConstructionScript`)