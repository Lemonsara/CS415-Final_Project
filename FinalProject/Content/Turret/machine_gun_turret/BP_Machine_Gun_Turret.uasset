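; Machine gun turret actor that automatically damages actors entering its Range component, ignoring other turrets and the first-person character.
; Overlap events maintain the EnemyInRange array, which a one-second polling loop watches until a target appears.
; AttackRound then repeatedly applies damage to the first entry on a short delay, and stops without resuming polling once the array empties.
; Turret rotation toward targets is unfinished, left in disconnected nodes.
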(event `self.ReceiveBeginPlay`
  (`KismetArrayLibrary.Array_Clear` (`self.enemy_in_range`))
  (`self.check`))

(event `check`
  (`KismetSystemLibrary.Delay` 1.0)
  (if (`KismetArrayLibrary.Array_IsEmpty` (`self.enemy_in_range`))
    (`self.check`)
    (else
      (`self.AttackRound`))))

(event `AttackRound`
  (bind _output (`|GetArrayItem` (`self.enemy_in_range`)))
  (`KismetSystemLibrary.PrintString` "attack round")
  (if (`KismetArrayLibrary.Array_IsEmpty` (`self.enemy_in_range`))
    (`KismetSystemLibrary.PrintString` "no enemy in the range")
    (else
      (`KismetSystemLibrary.PrintString` (`KismetSystemLibrary.GetDisplayName` _output))
      (`GameplayStatics.ApplyDamage` _output 10.0)
      (`KismetSystemLibrary.Delay` 0.2)
      (`self.AttackRound`))))

(event `self.range.OnComponentBeginOverlap`
  (params (OverlappedComponent :type "PrimitiveComponent Object Reference") (OtherActor :type "Actor Object Reference") (OtherComp :type "PrimitiveComponent Object Reference") (OtherBodyIndex :type Integer) (bFromSweep :type Boolean) (SweepResult :type "HitResult Structure (by ref)"))
  (cast `/Game/Turret/machine_gun_turret/BP_Machine_Gun_Turret` OtherActor
    (:`CastFailed`
      (cast `/Game/FirstPerson/Blueprints/BP_FirstPersonCharacter` OtherActor
        (:`CastFailed`
          (`KismetArrayLibrary.Array_Add` (`self.enemy_in_range`))
          (`KismetSystemLibrary.PrintString` "add")
          (`KismetSystemLibrary.PrintString` (`KismetSystemLibrary.GetDisplayName` OtherActor)))))))

(event `self.range.OnComponentEndOverlap`
  (params (OverlappedComponent :type "PrimitiveComponent Object Reference") (OtherActor :type "Actor Object Reference") (OtherComp :type "PrimitiveComponent Object Reference") (OtherBodyIndex :type Integer))
  (cast `/Game/FirstPerson/Blueprints/BP_FirstPersonCharacter` OtherActor
    (:`CastFailed`
      (`KismetArrayLibrary.Array_RemoveItem` (`self.enemy_in_range`)))))

(fn `UserConstructionScript`)